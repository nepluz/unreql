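; BP_door is a locked door that the player opens by spending a key.
; When a BP_ThirdPersonCharacter enters the Box trigger with at least one key in NombreDeClefs, it loses one key and the door-open call fires.
; The door_open event raises the PlSecretDoor01 component in one instant, unswept offset and disables the Box's overlap events.
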(event `self.Box.OnComponentBeginOverlap`
  (params (OverlappedComponent :type "PrimitiveComponent Object Reference") (OtherActor :type "Actor Object Reference") (OtherComp :type "PrimitiveComponent Object Reference") (OtherBodyIndex :type Integer) (bFromSweep :type Boolean) (SweepResult :type "HitResult Structure (by ref)"))
  (bind _asbp_third_person_character (cast `/Game/ThirdPerson/Blueprints/BP_ThirdPersonCharacter` OtherActor))
  (bind _nombre_de_clefs (`/Game/ThirdPerson/Blueprints/BP_ThirdPersonCharacter.nombre_de_clefs` _asbp_third_person_character))
  (if (> _nombre_de_clefs 0)
    (set `/Game/ThirdPerson/Blueprints/BP_ThirdPersonCharacter.nombre_de_clefs` (- _nombre_de_clefs 1) _asbp_third_person_character)
    (`self.door_open`)))

(event `door_open`
  (`SceneComponent.K2_AddLocalOffset` (`self.Pl_secretDoor_01`) (0.0 0.0 250.0) false false)
  (set `PrimitiveComponent.bGenerateOverlapEvents` false (`self.Box`)))

(fn `UserConstructionScript`)