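; BP_Vitesse is a speed power-up pickup whose PlPowerUp04 component spins continuously, a fixed step per tick.
; When an actor implementing NewInterface overlaps its Box, it sends that actor PickupAccelerationMessage and destroys itself.
; The receiver handles the speed effect; the walk-speed and ZoneMortAcitvationMessage nodes in this graph are unconnected and never run.
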(event `self.ReceiveTick`
  (params (DeltaSeconds :type "Float (single-precision)"))
  (`SceneComponent.K2_AddLocalRotation` (`self.Pl_PowerUp_04`) (struct :`Yaw` 5.0) false false))

(event `self.Box.OnComponentBeginOverlap`
  (params (OverlappedComponent :type "PrimitiveComponent Object Reference") (OtherActor :type "Actor Object Reference") (OtherComp :type "PrimitiveComponent Object Reference") (OtherBodyIndex :type Integer) (bFromSweep :type Boolean) (SweepResult :type "HitResult Structure (by ref)"))
  (if (`KismetSystemLibrary.DoesImplementInterface` OtherActor "/Game/NewInterface.NewInterface_C")
    (message `/Game/NewInterface.pickup_acceleration` OtherActor)
    (`self.K2_DestroyActor`)))

(fn `UserConstructionScript`)